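; BP_Door is a door actor whose material shows whether it is open, green for open and red for closed.
; The construction script creates a dynamic instance of DoorMaterial on DoorMesh and sets its LightColor parameter from IsOpenDoor.
; DoorDynMaterialOpenClose repeats that color update as a callable function.
; The event graph is inactive, and these graphs neither move the door nor change IsOpenDoor.
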(fn `DoorDynMaterialOpenClose`
  (bind _doordynmaterial (`self.DoorDynMaterial`))
  (if (`self.bIsOpenDoor`)
    (`MaterialInstanceDynamic.SetVectorParameterValue` _doordynmaterial "LightColor" (struct :`G` 1.0 :`A` 1.0))
    (return)
    (else
      (`MaterialInstanceDynamic.SetVectorParameterValue` _doordynmaterial "LightColor" (struct :`R` 1.0 :`A` 1.0))
      (return))))

(fn `UserConstructionScript`
  (bind _doordynmaterial (`self.DoorDynMaterial`))
  (bind _returnvalue (`PrimitiveComponent.CreateDynamicMaterialInstance` (`self.DoorMesh`) 0 (`self.DoorMaterial`) "None"))
  (set `self.DoorDynMaterial` _returnvalue)
  (if (`self.bIsOpenDoor`)
    (`MaterialInstanceDynamic.SetVectorParameterValue` _doordynmaterial "LightColor" (struct :`G` 1.0 :`A` 1.0))
    (else
      (`MaterialInstanceDynamic.SetVectorParameterValue` _doordynmaterial "LightColor" (struct :`R` 1.0 :`A` 1.0)))))