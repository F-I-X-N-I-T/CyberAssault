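; Placeable light actor pairing a rect light with a point light named for GI, presumably to supply fill or bounced light.
; The construction script pushes variables into both components: shape, barn doors and volumetric scattering for the rect light, falloff and indirect lighting for the point light.
; Both share one light color but keep separate intensity, radius and temperature settings.
; The event graph has no active logic.
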(fn `UserConstructionScript`
  (bind _dyn_rectlight (`self.Dyn_RectLight`))
  (bind _gi_pointlight (`self.GI_PointLight`))
  (`|ExecutionSequence`
    (:`then_0`
      ; RectLight
      (`LightComponent.SetIntensity` _dyn_rectlight (`self.DynIntensity`))
      (`LightComponent.SetLightColor` _dyn_rectlight (`self.DynLightColor`) true)
      (`RectLightComponent.SetSourceHeight` _dyn_rectlight (`self.DynSourceHeight`))
      (`RectLightComponent.SetSourceWidth` _dyn_rectlight (`self.DynSourceWidth`))
      (`RectLightComponent.SetBarnDoorAngle` _dyn_rectlight (`self.DynBarnDoorAngle`))
      (`RectLightComponent.SetBarnDoorLength` _dyn_rectlight (`self.DynBarnDoorLength`))
      (`LightComponent.SetVolumetricScatteringIntensity` _dyn_rectlight (`self.DynVolumetricScatteringIntensity`))
      (`LightComponent.SetUseTemperature` _dyn_rectlight (`self.DynUseTemperature`))
      (`LightComponent.SetTemperature` _dyn_rectlight (`self.DynTemperature`))
      (`LocalLightComponent.SetAttenuationRadius` _dyn_rectlight (`self.DynAttenuationRadius`)))
    (:`then_1`
      ; GI_PointLight
      (`LightComponent.SetIntensity` _gi_pointlight (`self.GIIntensity`))
      (`LightComponent.SetLightColor` _gi_pointlight (`self.DynLightColor`) true)
      (`LocalLightComponent.SetAttenuationRadius` _gi_pointlight (`self.GIAttenuationRadius`))
      (`LightComponent.SetUseTemperature` _gi_pointlight (`self.GIUseTemperature`))
      (`LightComponent.SetTemperature` _gi_pointlight (`self.GITemperature`))
      (`LightComponent.SetIndirectLightingIntensity` _gi_pointlight (`self.GIInderectLightingIntensity`))
      (`PointLightComponent.SetUseInverseSquaredFalloff` _gi_pointlight (`self.GIUseInverseSquaredFalloff`))
      (`PointLightComponent.SetLightFalloffExponent` _gi_pointlight (`self.GILightFalloffExponent`))
      (`PointLightComponent.SetInverseExposureBlend` _gi_pointlight (`self.GIInverseExposureBlend`))
      (`PointLightComponent.SetSourceRadius` _gi_pointlight (`self.GISourceRadius`)))))