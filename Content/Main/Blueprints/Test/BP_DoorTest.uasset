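; BP_DoorTest is a test door that slides along Z when an actor tagged Player1 enters its trigger, and returns when that actor leaves.
; BeginPlay caches the mesh's world location and derives the open location from the DoorOpenZ offset.
; Overlap events play or reverse a timeline that lerps the mesh between both locations without sweep.
; CanDoorOpen gates both opening and closing.
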(event `self.ReceiveBeginPlay`
  (set `self.DoorInitLocation` (`SceneComponent.K2_GetComponentLocation` (`self.DoorMesh`)))
  (set `self.DoorOpenLocation` (+ (`self.DoorInitLocation`) (`KismetMathLibrary.MakeVector` 0.0 0.0 (`self.DoorOpenZ`)))))

(event `self.DoorTrigger.OnComponentBeginOverlap`
  (params (OverlappedComponent :type "PrimitiveComponent Object Reference") (OtherActor :type "Actor Object Reference") (OtherComp :type "PrimitiveComponent Object Reference") (OtherBodyIndex :type Integer) (bFromSweep :type Boolean) (SweepResult :type "HitResult Structure (by ref)"))
  (if (`self.CanDoorOpen?`)
    (if (`self.ActorHasTag` OtherActor "Player1")
      (bind (_direction _opendoor) (`Timeline|TimelineDoorOpen` :!label _label)
        (:`Update`
          (`SceneComponent.K2_SetWorldLocation` (`self.DoorMesh`) (`KismetMathLibrary.VLerp` (`self.DoorInitLocation`) (`self.DoorOpenLocation`) _opendoor) false false))))))

(event `self.DoorTrigger.OnComponentEndOverlap`
  (params (OverlappedComponent :type "PrimitiveComponent Object Reference") (OtherActor :type "Actor Object Reference") (OtherComp :type "PrimitiveComponent Object Reference") (OtherBodyIndex :type Integer))
  (if (`self.CanDoorOpen?`)
    (if (`self.ActorHasTag` OtherActor "Player1")
      (goto _label :!via `Reverse`))))

(fn `UserConstructionScript`)